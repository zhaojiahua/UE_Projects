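; WXCameraMag is a player camera manager modeled on the ALS camera, with a skeletal mesh AnimBP for camera logic.
; On possess, it stores the pawn and passes it and the player controller to CameraMagAnimBP.
; For ALS_Char-tagged targets, it caches the pawn's pivot, first-person target, FOV, shoulder and trace data through interface calls; others use parent behavior.
; The custom path is unfinished, returning false with zeroed outputs and never applying the cached data.
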(event Custom|OnCtrlPossess
  (params (ctrledPawn :type Pawn%20Object%20Reference))
  (bind _output_get (Variables|Default|SetCtrled%20Pawn ctrledPawn))
  (bind _ascamera_mag_anim_bp (Utilities|Casting|CastToCameraMagAnimBP (Components|SkeletalMesh|GetAnimInstance (Variables|Default|GetSkeletalMesh))))
  (Variables|/Game/Blueprints/Globals/CameraMagAnimBP.CameraMagAnimBP_C|SetctrlledPawn _ascamera_mag_anim_bp _output_get)
  (Variables|/Game/Blueprints/Globals/CameraMagAnimBP.CameraMagAnimBP_C|SetplayerCtrl _ascamera_mag_anim_bp (Game|Player|GetOwningPlayerController)))

(event EventBeginPlay)

(event Collision|EventActorBeginOverlap
  (params (OtherActor :type Actor%20Object%20Reference)))

(event EventTick
  (params (DeltaSeconds :type Float%20%28single-precision%29)))

(fn ConstructionScript)

(fn BlueprintUpdateCamera
  (params (CameraTarget :type Actor%20Object%20Reference))
  (if (Actor|ActorHasTag CameraTarget "ALS_Char")
    (CallFunction|CustomCameraBehavior)
    (return "0, 0, 0" "0, 0, 0" 0.0 false)
    (else
      (bind (_newcameralocation _newcamerarotation _newcamerafov _returnvalue) (|CallParentFunction CameraTarget))
      (return _newcameralocation _newcamerarotation _newcamerafov _returnvalue))))

(fn CustomCameraBehavior
  (bind _ctrled_pawn (Variables|Default|GetCtrled%20Pawn))
  (Utilities|FlowControl|Sequence
    (:then_0
      ;[1 1 1] 从角色身上获取其相关的摄像机数据并临时存储在本地
      (bind _outtransform (Class|BPICameraInterface|BPIGetThirdPersonPivotTarget(Message) _ctrled_pawn))
      (LocalVariables|SettpCameraPivot _outtransform)
      (bind _outtarget (Class|BPICameraInterface|BPIGetFirstPersonCameraTarget(Message) _ctrled_pawn))
      (LocalVariables|SetfpCameraTargetLocation _outtarget)
      (bind (_thirdpersonfov _firstpersonfov _rightshoulder_) (Class|BPICameraInterface|BPIGetCameraParams(Message) _ctrled_pawn))
      (LocalVariables|SettpFOV _thirdpersonfov)
      (LocalVariables|SetfpFOV _firstpersonfov)
      (LocalVariables|SetrightShoulder? _rightshoulder_)
      (bind (_traceorg _traceradius) (Class|BPICameraInterface|BPIGetThirdPersonTraceParams(Message) _ctrled_pawn))
      (LocalVariables|SettraceOrgLocation _traceorg)
      (LocalVariables|SettraceRadius _traceradius))))

(fn BPIGetCameraParams
  (return 0.0 0.0 false))

(fn BPIGetFirstPersonCameraTarget
  (return "0, 0, 0"))

(fn BPIGetThirdPersonPivotTarget
  (return ""))

(fn BPIGetThirdPersonTraceParams
  (return "0, 0, 0" 0.0 "TraceTypeQuery1"))