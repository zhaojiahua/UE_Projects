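; WXChar_BP is a character Blueprint that supplies camera placement data through BPI getter functions.
; The third-person pivot averages the head and root sockets and uses the actor's rotation, while the trace origin switches between left and right shoulder sockets.
; First-person view uses a dedicated mesh socket, and both views return a fixed field of view.
; Its event graphs hold only disabled placeholder nodes.
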(event EventBeginPlay
  (|CallParentFunction) ; This node is disabled and will not be called.\nDrag off pins to build functionality.
)

(event Collision|EventActorBeginOverlap
  (params (OtherActor :type Actor%20Object%20Reference))
  (|CallParentFunction OtherActor) ; This node is disabled and will not be called.\nDrag off pins to build functionality.
)

(event EventTick
  (params (DeltaSeconds :type Float%20%28single-precision%29))
  (|CallParentFunction DeltaSeconds) ; This node is disabled and will not be called.\nDrag off pins to build functionality.
)

(fn ConstructionScript
  (|CallParentFunction))

(fn BPIGetThirdPersonTraceParams
  (bind _mesh (Variables|Character|GetMesh))
  ;[1 1 1] 第三人称视角下的左右肩相机位置
  (if (Variables|Default|GetrightShoulder?)
    (return (Transformation|GetSocketLocation _mesh "ThirdPersonCameraTrace_R") 1e+01 "TraceTypeQuery1")
    (else
      (return (Transformation|GetSocketLocation _mesh "ThirdPersonCameraTrace_L") 1e+01 "TraceTypeQuery1"))))

(fn BPIGetThirdPersonPivotTarget
  (bind _mesh (Variables|Character|GetMesh))
  ;[1 1 1] 第三人称下相机所在人物下的锚点位置(及旋转信息)
  (return (Math|Transform|MakeTransform (Math|Vector|GetVectorArrayAverage (Utilities|Array|MakeArray (Transformation|GetSocketLocation _mesh "HeadEnd_M") (Transformation|GetSocketLocation _mesh "Root_M"))) (Transformation|GetActorRotation))))

(fn BPIGetFirstPersonCameraTarget
  ;[1 1 1] 第一人称摄像机位置
  (return (Transformation|GetSocketLocation (Variables|Character|GetMesh) "FirstPersonCameraSocket")))

(fn BPIGetCameraParams
  (return 9e+01 9e+01))