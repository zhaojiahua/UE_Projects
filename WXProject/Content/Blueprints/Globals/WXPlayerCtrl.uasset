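; Player controller that turns Enhanced Input actions into pawn movement and look rotation.
; It adds the WX input mapping context on BeginPlay and passes each possessed pawn to the WXCameraMag camera manager.
; Movement follows control rotation, scaled by Movespeed, with each axis boosted and clamped by FixDiagonalMoveValue to correct diagonal input.
; Look input drives yaw and pitch scaled by Sensitivity.
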(event EventBeginPlay
  (Input|AddMappingContext (PlayerController|LocalPlayerSubsystems|GetEnhancedInputLocalPlayerSubsystem) "/Game/Inputs/WXInputMapping.WXInputMapping" 0 "(bIgnoreAllPressedKeysUntilRelease=True,bForceImmediately=False,bNotifyUserSettings=False)"))

(event EventTick
  (params (DeltaSeconds :type Float%20%28single-precision%29)))

(event EventPossess
  (params (PossessedPawn :type Pawn%20Object%20Reference))
  (bind _aswxcamera_mag (Utilities|Casting|CastToWXCameraMag (Variables|Default|GetPlayerCameraManager)))
  (Default|OnCtrlPossess _aswxcamera_mag PossessedPawn))

(event Input|EnhancedActionEvents|EnhancedInputActionInAc_MoveFB
  (params (ActionValue :type Float%20%28double-precision%29) (ElapsedSeconds :type Float%20%28double-precision%29) (TriggeredSeconds :type Float%20%28double-precision%29) (InputAction :type Input%20Action%20Object%20Reference :default "/Game/Inputs/InAc_MoveFB.InAc_MoveFB"))
  (Pawn|Input|AddMovementInput (Pawn|GetControlledPawn) (Math|Vector|GetForwardVector (Pawn|GetControlRotation :!class /Script/Engine.Controller)) (* (CallFunction|FixDiagonalMoveValue ActionValue) (Variables|Default|Getmovespeed)) false))

(event Input|EnhancedActionEvents|EnhancedInputActionInAc_MoveRL
  (params (ActionValue :type Float%20%28double-precision%29) (ElapsedSeconds :type Float%20%28double-precision%29) (TriggeredSeconds :type Float%20%28double-precision%29) (InputAction :type Input%20Action%20Object%20Reference :default "/Game/Inputs/InAc_MoveRL.InAc_MoveRL"))
  (Pawn|Input|AddMovementInput (Pawn|GetControlledPawn) (Math|Vector|GetRightVector (Pawn|GetControlRotation :!class /Script/Engine.Controller)) (* (Variables|Default|Getmovespeed) (CallFunction|FixDiagonalMoveValue ActionValue)) false))

(event Input|EnhancedActionEvents|EnhancedInputActionInAc_LookUDRL
  (params (ActionValue :type Vector%202D%20Structure) (ElapsedSeconds :type Float%20%28double-precision%29) (TriggeredSeconds :type Float%20%28double-precision%29) (InputAction :type Input%20Action%20Object%20Reference :default "/Game/Inputs/InAc_LookUDRL.InAc_LookUDRL"))
  (bind _sensitivity (Variables|Default|Getsensitivity))
  (Class|PlayerController|AddYawInput (* (.x ActionValue) _sensitivity))
  (Class|PlayerController|AddPitchInput (* (.y ActionValue) _sensitivity)))

(fn ConstructionScript)

(fn FixDiagonalMoveValue
  (params (inV :type Float%20%28double-precision%29))
  (return (Math|Float|Clamp(Float) (* inV (Math|Float|MapRangeClamped (Math|Float|Absolute(Float) inV) 0.0 0.6 1.0 1.2)) -1.0)))