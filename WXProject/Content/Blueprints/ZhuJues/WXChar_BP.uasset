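; Playable-style character Blueprint (WXChar) that adds held props, overlay-specific montages and camera sockets to its parent's overlay, mantle and ragdoll system.
; OverlayState picks the weapon or prop attached to a hand socket, refreshed on overlay changes, mantling and ragdoll end, and cleared on ragdoll start.
; It also selects low-mantle and get-up montages; Tick drives the bow's draw from an animation curve.
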(event EventBeginPlay
  (|CallParentFunction) ; This node is disabled and will not be called.\nDrag off pins to build functionality.
)

(event Collision|EventActorBeginOverlap
  (params (OtherActor :type Actor%20Object%20Reference))
  (|CallParentFunction OtherActor) ; This node is disabled and will not be called.\nDrag off pins to build functionality.
)

(event EventTick
  (params (DeltaSeconds :type Float%20%28single-precision%29))
  (|CallParentFunction DeltaSeconds)
  (AboutOverlays|UpdateHeldObjectAnimations))

(fn ConstructionScript
  (|CallParentFunction))

(fn BPIGetThirdPersonTraceParams
  (bind _mesh (Variables|Character|GetMesh))
  ;[1 1 1] 第三人称视角下的左右肩相机位置
  (if (Variables|Default|GetrightShoulder?)
    (return (Transformation|GetSocketLocation _mesh "ThirdPersonCameraTrace_R") 1e+01 "TraceTypeQuery1")
    (else
      (return (Transformation|GetSocketLocation _mesh "ThirdPersonCameraTrace_L") 1e+01 "TraceTypeQuery1"))))

(fn BPIGetThirdPersonPivotTarget
  (bind _mesh (Variables|Character|GetMesh))
  ;[1 1 1] 第三人称下相机所在人物下的锚点位置(及旋转信息)
  (return (Math|Transform|MakeTransform (Math|Vector|GetVectorArrayAverage (Utilities|Array|MakeArray (Transformation|GetSocketLocation _mesh "HeadEnd_M") (Transformation|GetSocketLocation _mesh "Root_M"))) (Transformation|GetActorRotation))))

(fn BPIGetFirstPersonCameraTarget
  ;[1 1 1] 第一人称摄像机位置
  (return (Transformation|GetSocketLocation (Variables|Character|GetMesh) "FirstPersonCameraSocket")))

(fn GetMantleAssetbyMantleType
  (params (mantleType :type ALS_MantleType%20Enum :default "NewEnumerator0"))
  (bind _mantle_1m_lh (Variables|Default|Getmantle_1m_LH))
  (bind _mantle_1m_rh (Variables|Default|Getmantle_1m_RH))
  (switch Utilities|FlowControl|Switch|SwitchonALS_MantleType mantleType
    (:NewEnumerator0
      _)
    (:NewEnumerator1
      (switch Utilities|FlowControl|Switch|SwitchonALS_OverlayState (Variables|Default|GetoverlayState)
        (:NewEnumerator6
          _)
        (:NewEnumerator7
          _)
        (:NewEnumerator8
          _)
        (:NewEnumerator9
          (return _mantle_1m_lh))
        (:NewEnumerator10
          (return (Variables|Default|Getmantle_1m_2H)))
        (:NewEnumerator11
          (return _mantle_1m_rh))
        (:NewEnumerator12
          (return _mantle_1m_rh))
        (:NewEnumerator13
          (return _mantle_1m_rh))
        (:NewEnumerator14
          (return _mantle_1m_lh))
        (:NewEnumerator15
          (return _mantle_1m_lh))
        (:NewEnumerator16
          (return _mantle_1m_rh))
        (:NewEnumerator17
          (return (Variables|Default|Getmantle_1m_box)))
        (:NewEnumerator18
          (return (Variables|Default|Getmantle_1m_LH))))
      (return (Variables|Default|Getmantle_1m_default)))
    (:NewEnumerator5
      _))
  (return (Variables|Default|Getmantle_2m_default)))

(fn GetRollAnimontage
  (switch Utilities|FlowControl|Switch|SwitchonALS_OverlayState (Variables|Default|GetoverlayState)
    (:NewEnumerator6
      (return (Variables|Default|GetlandRollDefault)))))

(fn UpdateHeldObjects
  (switch Utilities|FlowControl|Switch|SwitchonALS_OverlayState (Variables|Default|GetoverlayState)
    (:NewEnumerator6
      (AboutOverlays|ClearHeldObject :!label _label))
    (:NewEnumerator7
      (goto _label))
    (:NewEnumerator8
      (goto _label))
    (:NewEnumerator9
      (goto _label))
    (:NewEnumerator10
      (goto _label))
    (:NewEnumerator11
      (AboutOverlays|AttachtoHand "/Game/Propertys/Guns/Rifles/M4A1.M4A1" 0 0 "VB Wrist_R" (Math|Transform|MakeTransform "17.701422,-5.270142,-0.575866" "-8.333744,9.916456,-65.951393" "0.850000,0.850000,0.850000")))
    (:NewEnumerator12
      (AboutOverlays|AttachtoHand "/Game/Propertys/Guns/Pistols/DesertEagle.DesertEagle" 0 0 "VB Wrist_R" (Math|Transform|MakeTransform "8.538848,-5.008750,-2.299222" "-10.377074,10.349555,-81.401781" "1.100000,1.100000,1.100000")))
    (:NewEnumerator13
      (AboutOverlays|AttachtoHand "/Game/Propertys/Guns/Pistols/USP.USP" 0 0 "VB Wrist_R" (Math|Transform|MakeTransform "10.894850,-2.794449,-2.758950" "-12.479755,13.222896,-72.800376" "1.150000,1.150000,1.150000")))
    (:NewEnumerator14
      (AboutOverlays|AttachtoHand 0 "/Game/Propertys/Bows/recBOW.recBOW" "/Game/Propertys/Bows/Bow_AnimBP.Bow_AnimBP_C" "VB Wrist_L" (Math|Transform|MakeTransform "-7.317570,2.671593,2.526200" "-5.759765,13.855842,112.390000" "1.150000,1.150000,1.150000")))
    (:NewEnumerator15
      (AboutOverlays|AttachtoHand "/Game/Propertys/Torchs/Torch01.Torch01" 0 0 "VB Wrist_L" (Math|Transform|MakeTransform "-4.503108,-2.260070,3.299913" "0.000000,27.250278,91.786157" "0.800000,0.800000,0.800000")))
    (:NewEnumerator16
      (AboutOverlays|AttachtoHand "/Game/Propertys/Binoculars/Binoculars.Binoculars" 0 0 "VB Wrist_R" (Math|Transform|MakeTransform "7.109426,-5.064208,-11.224221" "-58.645633,-18.478131,40.424513" "0.800000,0.800000,0.800000")))
    (:NewEnumerator17
      (AboutOverlays|AttachtoHand "/Game/Propertys/Boxes/Box.Box" 0 0 "VB Wrist_R" (Math|Transform|MakeTransform "-12.082709,-12.454942,-27.067217" "1.967247,136.033129,0.000000" "2.254760,2.254760,2.254760")))
    (:NewEnumerator18
      (AboutOverlays|AttachtoHand "/Game/Propertys/Barrels/Barrel01.Barrel01" 0 0 "VB Wrist_L" (Math|Transform|MakeTransform "-6.824159,-5.532469,23.954920" "0.000000,0.000000,8.619527")))))

(fn ClearHeldObject
  (bind _skeletalmesh (Variables|Default|GetSkeletalMesh))
  (Components|StaticMesh|SetStaticMesh (Variables|Default|GetStaticMesh) 0)
  (Components|SkeletalMesh|SetSkeletalMeshAsset _skeletalmesh 0)
  (Class|SkeletalMeshComponent|SetAnimClass _skeletalmesh))

(fn AttachtoHand
  (params (inStaticMesh :type Static%20Mesh%20Object%20Reference) (inSkeletalMesh :type Skeletal%20Mesh%20Object%20Reference) (inAnimClass :type Object%20Class%20Reference) (slotName :type Name) (offset :type Transform))
  (bind _skeletalmesh (Variables|Default|GetSkeletalMesh))
  (bind _heldobjectsroot (Variables|Default|GetHeldObjectsRoot))
  (Utilities|FlowControl|Sequence
    (:then_0
      (AboutOverlays|ClearHeldObject))
    (:then_1
      (bind _instaticmesh (LocalVariables|GetinStaticMesh)
        (:then
          (Components|StaticMesh|SetStaticMesh (Variables|Default|GetStaticMesh) _instaticmesh))
        (:else)))
    (:then_2
      (bind _inskeletalmesh (LocalVariables|GetinSkeletalMesh)
        (:then
          (Components|SkeletalMesh|SetSkeletalMeshAsset _skeletalmesh _inskeletalmesh)
          (bind _inanimclass (LocalVariables|GetinAnimClass)
            (:then
              (Class|SkeletalMeshComponent|SetAnimClass _skeletalmesh _inanimclass))
            (:else)))
        (:else)))
    (:then_3
      (Transformation|AttachComponentToComponent _heldobjectsroot (Variables|Character|GetMesh) slotName "KeepRelative" "KeepRelative" "KeepRelative" true)
      (Transformation|SetRelativeTransform _heldobjectsroot offset false false))))

(fn UpdateHeldObjectAnimations
  (switch Utilities|FlowControl|Switch|SwitchonALS_OverlayState (Variables|Default|GetoverlayState)
    (:NewEnumerator14
      (bind _asbow_anim_bp (Utilities|Casting|CastToBow_AnimBP (Components|SkeletalMesh|GetAnimInstance (Variables|Default|GetSkeletalMesh))))
      (Variables|/Game/Propertys/Bows/Bow_AnimBP.Bow_AnimBP_C|Setdraw _asbow_anim_bp (CallFunction|GetAnimCurveValue "Enable_SpineRotation")))))

(fn OnOverlayStateChanged
  (params (overlayState :type ALS_OverlayState%20Enum :default "NewEnumerator6"))
  (|CallParentFunction overlayState)
  (AboutOverlays|UpdateHeldObjects))

(fn MantleStart
  (params (mantleHeight :type Float%20%28double-precision%29) (worldMantleLedge :type ALS%20Component%20and%20Transform%20Structure) (mantleType :type ALS_MantleType%20Enum :default "NewEnumerator0"))
  (|CallParentFunction mantleHeight worldMantleLedge mantleType)
  (switch Utilities|FlowControl|Switch|SwitchonALS_MantleType (Variables|Default|GetmantleType)
    (:NewEnumerator0
      _)
    (:NewEnumerator5
      _))
  (AboutOverlays|UpdateHeldObjects))

(fn MantleEnd
  (|CallParentFunction)
  (AboutOverlays|UpdateHeldObjects))

(fn GetGetupMontage
  (params (faceup? :type Boolean))
  (if faceup?
    (switch Utilities|FlowControl|Switch|SwitchonALS_OverlayState (Variables|Default|GetoverlayState)
      (:NewEnumerator6
        _)
      (:NewEnumerator7
        _)
      (:NewEnumerator8
        _)
      (:NewEnumerator9
        (return "/Game/Characters/BaseMales/Animations/Actions/WX_CLF_GetUp_Back_Montage_LH.WX_CLF_GetUp_Back_Montage_LH"))
      (:NewEnumerator10
        (return "/Game/Characters/BaseMales/Animations/Actions/WX_CLF_GetUp_Back_Montage_2H.WX_CLF_GetUp_Back_Montage_2H"))
      (:NewEnumerator11
        (return "/Game/Characters/BaseMales/Animations/Actions/WX_CLF_GetUp_Back_Montage_RH.WX_CLF_GetUp_Back_Montage_RH"))
      (:NewEnumerator12
        (return "/Game/Characters/BaseMales/Animations/Actions/WX_CLF_GetUp_Back_Montage_RH.WX_CLF_GetUp_Back_Montage_RH"))
      (:NewEnumerator13
        (return "/Game/Characters/BaseMales/Animations/Actions/WX_CLF_GetUp_Back_Montage_RH.WX_CLF_GetUp_Back_Montage_RH"))
      (:NewEnumerator14
        (return "/Game/Characters/BaseMales/Animations/Actions/WX_CLF_GetUp_Back_Montage_LH.WX_CLF_GetUp_Back_Montage_LH"))
      (:NewEnumerator15
        (return "/Game/Characters/BaseMales/Animations/Actions/WX_CLF_GetUp_Back_Montage_LH.WX_CLF_GetUp_Back_Montage_LH"))
      (:NewEnumerator16
        (return "/Game/Characters/BaseMales/Animations/Actions/WX_CLF_GetUp_Back_Montage_RH.WX_CLF_GetUp_Back_Montage_RH"))
      (:NewEnumerator17
        (return "/Game/Characters/BaseMales/Animations/Actions/WX_CLF_GetUp_Back_Montage_2H.WX_CLF_GetUp_Back_Montage_2H"))
      (:NewEnumerator18
        (return "/Game/Characters/BaseMales/Animations/Actions/WX_CLF_GetUp_Back_Montage_LH.WX_CLF_GetUp_Back_Montage_LH")))
    (return "/Game/Characters/BaseMales/Animations/Actions/WX_CLF_GetUp_Back_Montage_Default.WX_CLF_GetUp_Back_Montage_Default")
    (else
      (switch Utilities|FlowControl|Switch|SwitchonALS_OverlayState (Variables|Default|GetoverlayState)
        (:NewEnumerator6
          _)
        (:NewEnumerator7
          _)
        (:NewEnumerator8
          _)
        (:NewEnumerator9
          (return "/Game/Characters/BaseMales/Animations/Actions/WX_CLF_GetUp_Front_Montage_LH.WX_CLF_GetUp_Front_Montage_LH"))
        (:NewEnumerator10
          (return "/Game/Characters/BaseMales/Animations/Actions/WX_CLF_GetUp_Front_Montage_2H.WX_CLF_GetUp_Front_Montage_2H"))
        (:NewEnumerator11
          (return "/Game/Characters/BaseMales/Animations/Actions/WX_CLF_GetUp_Front_Montage_RH.WX_CLF_GetUp_Front_Montage_RH"))
        (:NewEnumerator12
          (return "/Game/Characters/BaseMales/Animations/Actions/WX_CLF_GetUp_Front_Montage_RH.WX_CLF_GetUp_Front_Montage_RH"))
        (:NewEnumerator13
          (return "/Game/Characters/BaseMales/Animations/Actions/WX_CLF_GetUp_Front_Montage_RH.WX_CLF_GetUp_Front_Montage_RH"))
        (:NewEnumerator14
          (return "/Game/Characters/BaseMales/Animations/Actions/WX_CLF_GetUp_Front_Montage_LH.WX_CLF_GetUp_Front_Montage_LH"))
        (:NewEnumerator15
          (return "/Game/Characters/BaseMales/Animations/Actions/WX_CLF_GetUp_Front_Montage_LH.WX_CLF_GetUp_Front_Montage_LH"))
        (:NewEnumerator16
          (return "/Game/Characters/BaseMales/Animations/Actions/WX_CLF_GetUp_Front_Montage_RH.WX_CLF_GetUp_Front_Montage_RH"))
        (:NewEnumerator17
          (return "/Game/Characters/BaseMales/Animations/Actions/WX_CLF_GetUp_Front_Montage_2H.WX_CLF_GetUp_Front_Montage_2H"))
        (:NewEnumerator18
          (return "/Game/Characters/BaseMales/Animations/Actions/WX_CLF_GetUp_Front_Montage_LH.WX_CLF_GetUp_Front_Montage_LH")))
      (return "/Game/Characters/BaseMales/Animations/Actions/WX_CLF_GetUp_Front_Montage_Default.WX_CLF_GetUp_Front_Montage_Default"))))

(fn RagdollStart
  (AboutOverlays|ClearHeldObject)
  (|CallParentFunction))

(fn RagdollEnd
  (|CallParentFunction)
  (AboutOverlays|UpdateHeldObjects))